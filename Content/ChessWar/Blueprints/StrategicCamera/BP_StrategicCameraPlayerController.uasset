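; Player controller for a strategy-style camera that moves, rotates and zooms the controlled pawn's view, with features toggled by flags.
; Initialize caches and angles the spring arm under the pawn's root.
; Axis inputs and Tick-polled mouse drags and screen-edge scrolling feed shared MoveActor and RotateActor helpers.
; Wheel and gamepad zoom set a target arm length that Tick interpolates toward; Tick also optionally shows the cursor only during mouse movement.
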(event `Initialize`
  (bind _returnvalue (`self.K2_GetPawn`))
  (bind _springarm (`self.SpringArm`))
  (`|ExecutionSequence`
    (:`then_0`
      ;[1 1 1] Cast Spring Arm Component from Player Pawn
      (`/Engine/EditorBlueprintResources/StandardMacros.IsValid` _returnvalue
        (:`Is Valid`
          (set `self.SpringArm` (cast `SpringArmComponent` (`SceneComponent.GetChildComponent` (`self.K2_GetRootComponent` _returnvalue) 0) :!pure true)))))
    (:`then_1`
      ;[1 1 1] Initialize Zoom Position If Zoom Unchecked
      (if (not (`self.Zoom`))
        (set `SpringArmComponent.TargetArmLength` (`self.ZoomPosition`) (`self.SpringArm`))))
    (:`then_2`
      ;[1 1 1] Set Initial Angle Rotation for Spring Arm Camera
      (if (`self.PitchOnZoom`)
        (bind _output_get (set `self.Iteration` (/ (- (`self.ZoomMax`) (`self.ZoomMin`)) (`self.SpeedZoom`))))
        (`SceneComponent.K2_SetRelativeRotation` (`self.SpringArm`) (`KismetMathLibrary.MakeRotator` 0.0 (* _output_get -4.0)) false false)
        (else
          (`/Engine/EditorBlueprintResources/StandardMacros.IsValid` _springarm
            (:`Is Valid`
              (`SceneComponent.K2_SetRelativeRotation` _springarm (`KismetMathLibrary.MakeRotator` 0.0 (`self.InitialAngleIfNoPitchOnZoom`)) false false))))))))

(event `InputAxis|Right`
  (params (AxisValue :type "Float (single-precision)"))
  ;[1 1 1] Move Forward and Move Right with key
  (if (`self.Move`) :!label _label
    (`ChessWarBPFunctionLibrary.MoveActor` (`self.K2_GetPawn`) AxisValue (stale `InputAxis|Forward` AxisValue) 0.0 (`self.SpeedMoveWithKey`))))

(event `InputAxis|Forward`
  (params (AxisValue :type "Float (single-precision)"))
  ;[1 1 1] Move Forward and Move Right with key
  (goto _label))

(event `InputAxis|RotateYaw`
  (params (AxisValue :type "Float (single-precision)"))
  ;[1 1 1] Rotate
  (if (`self.Rotate`) :!label _label_2
    (if (`self.RotateInYaw`)
      (set `self.Yaw` AxisValue)
      (if (`self.RotateInPitch`)
        (set `self.Pitch` (stale `InputAxis|RotatePitch` AxisValue))))
    (`ChessWarBPFunctionLibrary.RotateActor` self (`self.K2_GetPawn`) (`self.Yaw`) (`self.Pitch`) (`self.SpeedRotate`))))

(event `InputAxis|RotatePitch`
  (params (AxisValue :type "Float (single-precision)"))
  ;[1 1 1] Rotate
  (goto _label_2))

(event `InputAction|ZoomIn`
  (params (Key :type "Key Structure"))
  ;[1 1 1] Zoom Mouse Wheel
  (:`Pressed`
    (if (`self.Zoom`)
      (bind _zoomposition (`ChessWarBPFunctionLibrary.ZoomOnCamera` self (`self.K2_GetPawn`) (`self.SpringArm`) (- 0.0 (`self.SpeedZoom`)) (`self.ZoomMin`) (`self.ZoomMax`) (`self.MinCameraAngle`) (`self.MaxCameraAngle`) (`self.PitchOnZoom`) (`self.ZoomOnMousePosition`)))
      (set `self.ZoomPosition` _zoomposition))))

(event `InputAction|ZoomOut`
  (params (Key :type "Key Structure"))
  ;[1 1 1] Zoom Mouse Wheel
  (:`Pressed`
    (if (`self.Zoom`)
      (bind _zoomposition (`ChessWarBPFunctionLibrary.ZoomOnCamera` self (`self.K2_GetPawn`) (`self.SpringArm`) (`self.SpeedZoom`) (`self.ZoomMin`) (`self.ZoomMax`) (`self.MinCameraAngle`) (`self.MaxCameraAngle`) (`self.PitchOnZoom`) false))
      (set `self.ZoomPosition` _zoomposition))))

(event `InputAxis|Zoom`
  (params (AxisValue :type "Float (single-precision)"))
  (bind _returnvalue (`KismetMathLibrary.FClamp` (+ (* AxisValue (`self.SpeedZoom`)) (`SpringArmComponent.TargetArmLength` (`self.SpringArm`))) (`self.ZoomMin`) (`self.ZoomMax`)))
  ;[1 1 1] Zoom GamePad
  (set `self.ZoomGamePadAxis` AxisValue)
  (if (`self.Zoom`)
    (if (== AxisValue 0.0)
      (bind (_direction _smooth_value) (`Timeline|Smooth Zoom` :!via `PlayFromStart`)
        (:`Update`
          (`/Engine/EditorBlueprintResources/StandardMacros.CompareFloat` (`self.ZoomGamePadAxis`)
            (:`>`
              (set `self.ZoomPosition` (+ _smooth_value _returnvalue)))
            (:`<`
              (set `self.ZoomPosition` (- _returnvalue _smooth_value)))))))))

(event `self.ReceiveTick`
  (params (DeltaSeconds :type "Float (single-precision)"))
  (bind (_locationx _locationy _returnvalue) (`self.GetMousePosition`))
  (bind _returnvalue_2 (`self.K2_GetPawn`))
  (bind (_sizex _sizey) (`self.GetViewportSize`))
  (bind (_deltax _deltay) (`self.GetInputMouseDelta`))
  (bind (_deltax_2 _deltay_2) (`self.GetInputMouseDelta`))
  (bind (_deltax_3 _deltay_3) (`self.GetInputMouseDelta`))
  (bind _moverightwithborder (`self.MoveRightWithBorder`))
  (bind _moveforwardwithborder (`self.MoveForwardWithBorder`))
  (bind _activezoneinborder (`self.ActiveZoneInBorder`))
  (bind _activezoneinborder_2 (`self.ActiveZoneInBorder`))
  (bind _speedmovewithborder (`self.SpeedMoveWithBorder`))
  (bind _springarm (`self.SpringArm`))
  (bind _returnvalue_3 (`KismetMathLibrary.FFloor` _locationx))
  (bind _returnvalue_4 (`KismetMathLibrary.FFloor` _locationy))
  (set `self.WorldDeltaSecond` DeltaSeconds)
  (`|ExecutionSequence`
    (:`then_0`
      ;[1 1 1] Rotate with Mouse
      (if (`self.RotateWithRightMouseButton`)
        (if (!= (`self.GetInputKeyTimeDown` "RightMouseButton") 0.0)
          (if (`self.RotateInYaw`)
            (set `self.Yaw` _deltax_3)
            (if (`self.RotateInPitch`)
              (set `self.Pitch` _deltay_3)))
          (`ChessWarBPFunctionLibrary.RotateActor` self (`self.K2_GetPawn`) (`self.Yaw`) (`self.Pitch`) (`self.SpeedRotateWithMouse`)))))
    (:`then_1`
      ;[1 1 1] Move Forward and Move Right with Mouse
      (if (`self.MoveWithMiddleMouseButton`)
        (if (!= (`self.GetInputKeyTimeDown` "MiddleMouseButton") 0.0)
          (`ChessWarBPFunctionLibrary.MoveActor` (`self.K2_GetPawn`) _deltax _deltay 0.0 (`self.SpeedMoveWithMouse`) true))))
    (:`then_2`
      ;[1 1 1] Smooth Zoom
      (if (`self.Zoom`)
        (`/Engine/EditorBlueprintResources/StandardMacros.IsValid` _springarm
          (:`Is Valid`
            (set `SpringArmComponent.TargetArmLength` (`KismetMathLibrary.FInterpTo` (`SpringArmComponent.TargetArmLength` (`self.SpringArm`)) (`self.ZoomPosition`) (`self.WorldDeltaSecond`) 4.0) _springarm)))))
    (:`then_3`
      ;[1 1 1] Move with Border Screen
      (if (and (`self.MoveWithScreenBorder`) _returnvalue)
        (`|ExecutionSequence`
          (:`then_0`
            (if (<= (- _sizex _activezoneinborder) _returnvalue_3)
              (`ChessWarBPFunctionLibrary.MoveActor` _returnvalue_2 _moverightwithborder 0.0 0.0 _speedmovewithborder) ; Right
            ))
          (:`then_1`
            (if (<= (- _sizey _activezoneinborder) _returnvalue_4)
              (`ChessWarBPFunctionLibrary.MoveActor` _returnvalue_2 0.0 _moveforwardwithborder 0.0 _speedmovewithborder true) ; Back
            ))
          (:`then_2`
            (if (<= _returnvalue_3 _activezoneinborder_2)
              (`ChessWarBPFunctionLibrary.MoveActor` _returnvalue_2 _moverightwithborder 0.0 0.0 _speedmovewithborder true) ; Left
            ))
          (:`then_3`
            (if (<= _returnvalue_4 _activezoneinborder_2)
              (`ChessWarBPFunctionLibrary.MoveActor` _returnvalue_2 0.0 _moveforwardwithborder 0.0 _speedmovewithborder) ; Forward
            )))))
    (:`then_4`
      ;[1 1 1] Is Mouse Activate only if movement
      (if (`self.MouseControlActiveOnMovement`)
        (if (or (!= (`KismetMathLibrary.Abs` _deltax_2) 0.0) (!= (`KismetMathLibrary.Abs` _deltay_2) 0.0))
          (if (not (`self.bShowMouseCursor`))
            (`self.ActivateMouse` true)
            (`WidgetBlueprintLibrary.SetInputMode_GameAndUIEx` self null))
          (elif (`self.bShowMouseCursor`)
            (`KismetSystemLibrary.Delay` (`self.DelayToHideMouseAfterMovement`))
            (`self.ActivateMouse` false)
            (if (`self.MouseControlActiveOnMovement`)
              (`WidgetBlueprintLibrary.SetInputMode_GameOnly` self))))))))

(event `InputAxis|Up`
  (params (AxisValue :type "Float (single-precision)"))
  ;[1 1 1] Move Up With Key
  (if (`self.MoveUpWithKey`)
    (`ChessWarBPFunctionLibrary.MoveActor` (`self.K2_GetPawn`) 0.0 0.0 AxisValue (`self.SpeedMoveWithKey`))))

(fn `ActivateMouse`
  (params (Enable :type Boolean))
  (bind _output_get (set `self.bShowMouseCursor` Enable))
  (bind _output_get_2 (set `self.bEnableClickEvents` _output_get))
  (set `self.bEnableMouseOverEvents` _output_get_2)
  (return))

(fn `UserConstructionScript`)