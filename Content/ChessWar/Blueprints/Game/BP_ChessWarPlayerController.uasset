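; Player controller for the ChessWar chess game, turning mouse and gamepad input into piece selection, board moves and HUD toggles.
; Mouse clicks trace under the cursor to select current-player pieces or target squares; gamepad input steps and confirms.
; Results broadcast through event dispatchers, with the game instance's touch-move rule restricting deselection and reselection.
; BeginPlay applies the game instance's mouse setting and spawns the countdown actor.
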(event `InputAction|Moves`
  (params (Key :type "Key Structure"))
  ;[1 1 1] Display HUD Elements
  (:`Pressed`
    (if (`self.IsMovesHiding`)
      (set `self.IsMovesHiding` false)
      (else
        (set `self.IsMovesHiding` true)))
    (bind _foundwidgets (`WidgetBlueprintLibrary.GetAllWidgetsOfClass` "/Game/ChessWar/Widgets/ChessWarGameHUD.ChessWarGameHUD_C"))
    (`/Game/ChessWar/Widgets/ChessWarGameHUD.Event Display Moves` (`|GetArrayItem` _foundwidgets) (not (`self.IsMovesHiding`)))))

(event `InputAction|Minimap`
  (params (Key :type "Key Structure"))
  ;[1 1 1] Display HUD Elements
  (:`Pressed`
    (if (`self.IsMinimapHiding`)
      (set `self.IsMinimapHiding` false)
      (else
        (set `self.IsMinimapHiding` true)))
    (bind _foundwidgets (`WidgetBlueprintLibrary.GetAllWidgetsOfClass` "/Game/ChessWar/Widgets/ChessWarGameHUD.ChessWarGameHUD_C"))
    (`/Game/ChessWar/Widgets/ChessWarGameHUD.Event Display Minimap` (`|GetArrayItem` _foundwidgets) (not (`self.IsMinimapHiding`)))))

(event `InputAction|GamepadTop`
  (params (Key :type "Key Structure"))
  ;[1 1 1] Pad Move Pushed Event
  (:`Pressed`
    (`self.PadMovePushed` (`self.IsSelectionOn`) (`self.SelectedPiece`) 0.0 -1.0)))

(event `InputAction|GamePadSelect`
  (params (Key :type "Key Structure"))
  (bind _selectedpiece (`self.SelectedPiece`))
  (bind (_returnvalue_x _returnvalue_y _returnvalue_z) (`KismetMathLibrary.BreakVector` (`self.K2_GetActorLocation` _selectedpiece)))
  ;[1 1 1] Move and Select Piece with pad
  (:`Pressed`
    (if (`self.IsSelectionOn`)
      (`self.BoardClicked` false _selectedpiece 0.0 0.0 _returnvalue_z)
      (else
        (`self.PieceClicked` (`self.SelectedPiece`) true)))))

(event `InputAction|GamepadBottom`
  (params (Key :type "Key Structure"))
  ;[1 1 1] Pad Move Pushed Event
  (:`Pressed`
    (`self.PadMovePushed` (`self.IsSelectionOn`) (`self.SelectedPiece`) 0.0 1.0)))

(event `InputAction|GamePadCancelSelect`
  (params (Key :type "Key Structure"))
  ;[1 1 1] Move and Select Piece with pad
  (:`Pressed`
    (if (not (`self.IsTouchMoveRule`))
      (`self.PieceClicked` null))))

(event `InputAction|GamepadRight`
  (params (Key :type "Key Structure"))
  ;[1 1 1] Pad Move Pushed Event
  (:`Pressed`
    (`self.PadMovePushed` (`self.IsSelectionOn`) (`self.SelectedPiece`) 1.0)))

(event `InputAction|GamepadtLeft`
  (params (Key :type "Key Structure"))
  ;[1 1 1] Pad Move Pushed Event
  (:`Pressed`
    (`self.PadMovePushed` (`self.IsSelectionOn`) (`self.SelectedPiece`) -1.0)))

(event `InputAction|Click`
  (params (Key :type "Key Structure"))
  (bind _hitresult (`self.GetHitResultUnderCursorByChannel` "TraceTypeQuery1"))
  ;[1 1 1] Move and select Piece with mouse
  (:`Pressed`
    (cast `/Game/ChessWar/Blueprints/Game/BP_Board` (`.HitActor` (`GameplayStatics.BreakHitResult` _hitresult))
      (:`then`
        ;;[1 1 1] Init Positions And Target
        (`self.InitPositionsAndTarget` (`.HitComponent` (`GameplayStatics.BreakHitResult` _hitresult)))
        ;;[1 1 1] Board Clicked Event
        (`self.BoardClicked` true (`self.SelectedPiece`) (`self.TargetX`) (`self.TargetY`) (`self.PosZ`))
        (if (not (`self.IsTouchMoveRule`))
          (`self.SetPieceSelected` null)))
      (:`CastFailed`
        (bind _asbp_chess_war_character (cast `/Game/ChessWar/Blueprints/Game/BP_ChessWarCharacter` (`.HitActor` (`GameplayStatics.BreakHitResult` _hitresult)))
          (:`then`
            ;;[1 1 1] Piece Clicked Event and Piece Clicket Event Fail
            (if (`self.IsSameColorOnSelectedPieceAndCurrentPlayer` _asbp_chess_war_character)
              (if (`self.IsTouchMoveRule`) :!label _label
                (if (not (`self.IsSelectionOn`))
                  (bind _selectedpiece (`self.SetPieceSelected` _asbp_chess_war_character :!label _label_2))
                  (`self.PieceClicked` _selectedpiece true))
                (else
                  (goto _label_2)))))
          (:`CastFailed`
            (goto _label)))))))

(event `self.ReceiveBeginPlay`
  ;[1 1 1] Apply Mouse Control and spawn CountDown
  (`|ExecutionSequence`
    (:`then_0`
      (set `self.ChessWarGameInstance` (cast `/Game/ChessWar/Blueprints/Game/BP_ChessWarGameInstance` (`GameplayStatics.GetGameInstance`) :!pure true)))
    (:`then_1`
      (bind _output_get (set `self.MouseControlActiveOnMovement` (`self.IsMouseActive`)))
      (bind _output_get_2 (set `self.RotateWithRightMouseButton` _output_get))
      (bind _output_get_3 (set `self.MoveWithMiddleMouseButton` _output_get_2))
      (`self.ActivateMouse` _output_get_3))
    (:`then_2`
      (bind _returnvalue (`|SpawnActorFromClass` "/Game/ChessWar/Blueprints/Game/BP_CountDown.BP_CountDown_C" (`KismetMathLibrary.MakeTransform` (0.0 0.0 0.0)) "Undefined" "OverrideRootScale" null null))
      (set `self.CountDown` _returnvalue))
    (:`then_3`
      (`parent.ReceiveBeginPlay`))))

(fn `InitPositionsAndTarget`
  (params (MeshComponent :type "SceneComponent Object Reference"))
  (bind (_returnvalue_x _returnvalue_y) (`KismetMathLibrary.BreakVector` (`SceneComponent.K2_GetComponentLocation` MeshComponent)))
  (set `self.TargetX` (`KismetMathLibrary.Conv_IntToDouble` (`KismetMathLibrary.Round` _returnvalue_x)))
  (set `self.TargetY` (`KismetMathLibrary.Conv_IntToDouble` (`KismetMathLibrary.Round` _returnvalue_y)))
  (set `self.PosZ` (+ (* (`KismetMathLibrary.Conv_IntToDouble` (`KismetMathLibrary.FFloor` (.z (`.BoxExtent` (`KismetSystemLibrary.GetComponentBounds` MeshComponent))))) 2.0) (`/Game/ChessWar/Blueprints/Game/BP_ChessWarGameInstance.CharacterOffsetMovement` (`self.ChessWarGameInstance`)))))

(fn `IsMouseActive`
  (returns (IsMouseActive :type Boolean))
  (return (`/Game/ChessWar/Blueprints/Game/BP_ChessWarGameInstance.IsMouseEnable` (`self.ChessWarGameInstance`))))

(fn `IsSameColorOnSelectedPieceAndCurrentPlayer`
  (params (SelectedPiece :type "ChessWarCharacter Object Reference"))
  (returns (IsSameColor :type Boolean))
  (return (== (`self.Color`) (`KismetMathLibrary.Conv_BoolToByte` (not (`ChessWarCharacter.bIsBlack` SelectedPiece))))))

(fn `IsTouchMoveRule`
  (returns (IsTouchMoveRule :type Boolean))
  (return (`/Game/ChessWar/Blueprints/Game/BP_ChessWarGameInstance.IsTouchMoveRule` (`self.ChessWarGameInstance`))))

(fn `SetPieceSelected`
  (params (NewSelectedPiece :type "/Game/ChessWar/Blueprints/Game/BP_ChessWarCharacter Object Reference"))
  (returns (SelectedPiece :type "/Game/ChessWar/Blueprints/Game/BP_ChessWarCharacter Object Reference"))
  (bind _selectedpiece (`self.SelectedPiece`)
    (:`then`
      (`/Game/ChessWar/Blueprints/Game/BP_ChessWarCharacter.SetSelected` _selectedpiece false))
    (:`else`
      _))
  (bind _output_get (set `self.SelectedPiece` NewSelectedPiece))
  (bind _selectedpiece_2 (`self.SelectedPiece`)
    (:`then`
      (set `self.LastSelectedPiece` _selectedpiece_2)
      (`/Game/ChessWar/Blueprints/Game/BP_ChessWarCharacter.SetSelected` _output_get true))
    (:`else`
      _))
  (return (`self.SelectedPiece`)))

(fn `UserConstructionScript`
  (`parent.UserConstructionScript`))