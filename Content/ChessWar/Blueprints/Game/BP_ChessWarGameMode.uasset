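; Game mode for the chess game that assigns player colours and runs turn order for player-vs-PC and local two-player matches.
; ChoosePlayerStart matches tagged PlayerStarts to Player 1's chosen colour, and BeginPlay gives the AI the opposite colour, then starts the first move and HUD countdowns.
; NextMove swaps current player and opponent, toggles their input, records turn state in the GameInstance, and blends views to the current player in local play.
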(event `self.ReceiveBeginPlay`
  (`KismetSystemLibrary.Delay` 0.0)
  (`|ExecutionSequence`
    (:`then_0`
      ;[1 1 1] Casting
      (set `self.ChessWarGameInstance` (cast `/Game/ChessWar/Blueprints/Game/BP_ChessWarGameInstance` (`GameplayStatics.GetGameInstance`) :!pure true))
      ;[1 1 1] Set AI Controller Color
      (`/Engine/EditorBlueprintResources/StandardMacros.IsValid` (`self.AIController`)
        (:`Is Valid`
          (if (`|EnumEquality` (`/Game/ChessWar/Blueprints/Game/BP_ChessWarPlayerController.Color` (cast `/Game/ChessWar/Blueprints/Game/BP_ChessWarPlayerController` (`GameplayStatics.GetPlayerController` 0) :!pure true)) "NewEnumerator1")
            (set `/Game/ChessWar/Blueprints/Game/BP_ChessWarAIController.Color` "NewEnumerator0" (`self.AIController`))
            (else
              (set `/Game/ChessWar/Blueprints/Game/BP_ChessWarAIController.Color` "NewEnumerator1" (`self.AIController`)))))))
    (:`then_1`
      ;[1 1 1] Lance le jeu
      (`self.NextMove` 0.0)
      (`self.InitCountdowns`)
      (`self.BeginMove` true))))

(fn `ChoosePlayerStart`
  (params (Player :type "Controller Object Reference"))
  (returns (ReturnValue :type "Actor Object Reference"))
  (locals (PlayerStart :type "PlayerStart Object Reference") (PlayerStarts :type "Array of PlayerStart Object Reference") (PlayerController :type "/Game/ChessWar/Blueprints/Game/BP_ChessWarPlayerController Object Reference"))
  (bind _player1color (`self.Player1Color`))
  (set `local.PlayerController` (cast `/Game/ChessWar/Blueprints/Game/BP_ChessWarPlayerController` Player :!pure true))
  (set `self.Player1Color` (`/Game/ChessWar/Blueprints/Game/BP_ChessWarGameInstance.Player1Color` (cast `/Game/ChessWar/Blueprints/Game/BP_ChessWarGameInstance` (`GameplayStatics.GetGameInstance`) :!pure true)))
  (bind _outactors (`GameplayStatics.GetAllActorsOfClass` "/Script/Engine.PlayerStart"))
  (bind _output_get (set `local.PlayerStarts` _outactors))
  ;[1 1 1] Get Player Start
  (for _array_element _output_get
    (if (== (`GameplayStatics.GetPlayerController` 0) (`local.PlayerController`))
      (bind _returnvalue (== (`PlayerStart.PlayerStartTag` _array_element) (`KismetStringLibrary.Conv_StringToName` (`|GetEnumeratorNameAsString` _player1color))))
      (if _returnvalue
        (set `/Game/ChessWar/Blueprints/Game/BP_ChessWarPlayerController.Color` (`self.Player1Color`) (`local.PlayerController`))
        (set `local.PlayerStart` _array_element :!label _label))
      (elif (not _returnvalue)
        (switch `/Game/ChessWar/Blueprints/Game/EColor` _player1color
          (:`NewEnumerator0`
            (set `/Game/ChessWar/Blueprints/Game/BP_ChessWarPlayerController.Color` "NewEnumerator1" (`local.PlayerController`))
            (goto _label))
          (:`NewEnumerator1`
            (set `/Game/ChessWar/Blueprints/Game/BP_ChessWarPlayerController.Color` "NewEnumerator0" (`local.PlayerController`))
            (goto _label))))))
  (return (`local.PlayerStart`)))

(fn `InitCountdowns`
  (locals (GameHUD :type "/Game/ChessWar/Widgets/ChessWarGameHUD Object Reference"))
  (bind _aicontroller (`self.AIController`))
  (bind _gamehud (`local.GameHUD`))
  (bind _gamehud_2 (`local.GameHUD`))
  (bind _currentplayer (`self.CurrentPlayer`))
  (bind _playercontroller2 (`self.PlayerController2`))
  (bind _foundwidgets (`WidgetBlueprintLibrary.GetAllWidgetsOfClass` "/Game/ChessWar/Widgets/ChessWarGameHUD.ChessWarGameHUD_C"))
  (set `local.GameHUD` (`|GetArrayItem` _foundwidgets))
  (`/Engine/EditorBlueprintResources/StandardMacros.IsValid` _currentplayer
    (:`Is Valid`
      (`/Game/ChessWar/Widgets/ChessWarGameHUD.Event Init Countdowns` _gamehud_2 _currentplayer))
    (:`Is Not Valid`
      (`/Game/ChessWar/Widgets/ChessWarGameHUD.Event Init Countdowns` _gamehud_2 _aicontroller)))
  (`/Engine/EditorBlueprintResources/StandardMacros.IsValid` _playercontroller2
    (:`Is Valid`
      (`/Game/ChessWar/Widgets/ChessWarGameHUD.Event Init Countdowns` _gamehud _playercontroller2))
    (:`Is Not Valid`
      (`/Game/ChessWar/Widgets/ChessWarGameHUD.Event Init Countdowns` _gamehud _aicontroller))))

(fn `NextMove`
  (params (CameraMvtDelay :type "Float (double-precision)"))
  (locals (BlendTime :type "Float (double-precision)"))
  (bind _currentplayer (`self.CurrentPlayer`))
  (bind _playercontroller2 (`self.PlayerController2`))
  (bind _currentplayer_2 (`self.CurrentPlayer`))
  (bind _playercontroller2_2 (`self.PlayerController2`))
  (bind _chesswargameinstance (`self.ChessWarGameInstance`))
  (bind _players (`/Game/ChessWar/Blueprints/Game/BP_ChessWarGameInstance.Players` _chesswargameinstance))
  (set `local.BlendTime` CameraMvtDelay)
  (`self.SetPlayers`)
  (`/Engine/EditorBlueprintResources/StandardMacros.IsValid` _playercontroller2
    (:`Is Valid`
      (`self.DisableInput` _playercontroller2 _playercontroller2)
      (`/Game/ChessWar/Blueprints/Game/BP_ChessWarPlayerController.SetPieceSelected` _playercontroller2 null))
    (:`Is Not Valid`
      _))
  (`/Engine/EditorBlueprintResources/StandardMacros.IsValid` _currentplayer
    (:`Is Valid`
      (`self.EnableInput` _currentplayer _currentplayer))
    (:`Is Not Valid`
      _))
  (switch `/Game/ChessWar/Blueprints/Game/EGameType` (`self.GameType`)
    (:`NewEnumerator0`
      _)
    (:`NewEnumerator1`
      (`PlayerController.SetViewTargetWithBlend` (`self.PlayerController2`) (`Controller.K2_GetPawn` _currentplayer) (`local.BlendTime`) "VTBlend_Linear" 0.0 false)
      (`PlayerController.SetViewTargetWithBlend` _currentplayer (`Controller.K2_GetPawn` _currentplayer) (`local.BlendTime`) "VTBlend_Linear" 0.0 false)))
  ;[1 1 1] Save In GameInstance
  (`/Engine/EditorBlueprintResources/StandardMacros.IsValid` _currentplayer_2
    (:`Is Valid`
      (set `/Game/ChessWar/Blueprints/Game/BP_ChessWarGameInstance.CurrentPlayer` _currentplayer_2 _chesswargameinstance)
      (`KismetArrayLibrary.Array_AddUnique` _players _currentplayer_2))
    (:`Is Not Valid`
      _))
  (`/Engine/EditorBlueprintResources/StandardMacros.IsValid` _playercontroller2_2
    (:`Is Valid`
      (`KismetArrayLibrary.Array_AddUnique` _players _playercontroller2_2))
    (:`Is Not Valid`
      _))
  (set `/Game/ChessWar/Blueprints/Game/BP_ChessWarGameInstance.Turn` (+ (`/Game/ChessWar/Blueprints/Game/BP_ChessWarGameInstance.Turn` _chesswargameinstance) 1) _chesswargameinstance))

(fn `SetPlayers`
  (bind _asbp_chess_war_player_controller (cast `/Game/ChessWar/Blueprints/Game/BP_ChessWarPlayerController` (`GameplayStatics.GetPlayerController` 0) :!pure true))
  (bind _asbp_chess_war_player_controller_2 (cast `/Game/ChessWar/Blueprints/Game/BP_ChessWarPlayerController` (`GameplayStatics.GetPlayerController` 1) :!pure true))
  (if (== (`self.CurrentPlayerColor`) (`/Game/ChessWar/Blueprints/Game/BP_ChessWarPlayerController.Color` _asbp_chess_war_player_controller))
    (set `self.CurrentPlayer` _asbp_chess_war_player_controller)
    (switch `/Game/ChessWar/Blueprints/Game/EGameType` (`self.GameType`)
      (:`NewEnumerator0`
        (set `self.PlayerController2` null))
      (:`NewEnumerator1`
        (set `self.PlayerController2` _asbp_chess_war_player_controller_2)))
    (else
      (set `self.PlayerController2` _asbp_chess_war_player_controller)
      (switch `/Game/ChessWar/Blueprints/Game/EGameType` (`self.GameType`)
        (:`NewEnumerator0`
          (set `self.CurrentPlayer` null))
        (:`NewEnumerator1`
          (set `self.CurrentPlayer` _asbp_chess_war_player_controller_2)))))
  (switch `/Game/ChessWar/Blueprints/Game/EColor` (`self.CurrentPlayerColor`)
    (:`NewEnumerator0`
      (set `self.CurrentPlayerColor` "NewEnumerator1"))
    (:`NewEnumerator1`
      (set `self.CurrentPlayerColor` "NewEnumerator0"))))

(fn `UserConstructionScript`)