(event `self.ReceiveActorBeginCursorOver`
  ;[1 1 1] Actions On Hover on Piece - Set decal visibility
  (`SceneComponent.SetVisibility` (`self.CircleDecal`) true false))

(event `self.ReceiveActorEndCursorOver`
  ;[1 1 1] Actions On Hover on Piece - Set decal visibility
  (if (not (`self.bIsSelected`))
    (`SceneComponent.SetVisibility` (`self.CircleDecal`) false false)))

(event `self.ReceiveBeginPlay`
  ;[1 1 1] Cast to game instance at beginplay
  (set `self.ChessWarGameInstance` (cast `/Game/ChessWar/Blueprints/Game/BP_ChessWarGameInstance` (`GameplayStatics.GetGameInstance`) :!pure true)))

(event `Spawned`
  (bind _chesswargameinstance (`self.ChessWarGameInstance`))
  (bind _returnvalue (* (`/Game/ChessWar/Blueprints/Game/BP_ChessWarGameInstance.CharacterOffsetMovement` _chesswargameinstance) -1.0))
  ;[1 1 1] Spawn Static Mesh, Set Dynamic Material and Parameters, Spawn Decal Circle
  (switch `/Game/ChessWar/Blueprints/Game/EPiecesLook` (`/Game/ChessWar/Blueprints/Game/BP_ChessWarGameInstance.PiecesLook` _chesswargameinstance)
    (:`NewEnumerator0`
      (bind _returnvalue_2 (`AddComponent|NODE_AddStaticMeshComponent-0` :`RelativeTransform` (`KismetMathLibrary.MakeTransform` (`KismetMathLibrary.MakeVector` 0.0 0.0 _returnvalue) (struct :`Yaw` -90.0))))
      (bind _output_get (set `self.StaticMeshComponent` _returnvalue_2))
      (bind _returnvalue_3 (`PrimitiveComponent.CreateDynamicMaterialInstance` _output_get 0 "/Game/ChessWar/Materials/Game/DefaultLook/M_Piece.M_Piece" "None"))
      (set `self.Material` _returnvalue_3)
      (`self.SetDefaultLook` (`self.EPieceType`)))
    (:`NewEnumerator1`
      (`SceneComponent.K2_SetRelativeLocation` (`self.Mesh`) (`KismetMathLibrary.MakeVector` 0.0 0.0 _returnvalue) false false)
      (bind _returnvalue_4 (`PrimitiveComponent.CreateDynamicMaterialInstance` (`self.Mesh`) 0 "/Game/MovementAnimsetPro/UE4_Mannequin/Materials/M_UE4Man_Body.M_UE4Man_Body" "None"))
      (set `self.Material` _returnvalue_4)
      (`self.SetFantasyLook` (`self.EPieceType`)))))

(event `ChangeType`
  (params (PieceType :type "EPiecesType Enum" :default "E_Bishop"))
  ;[1 1 1] Change Piece Type
  (bind _output_get (set `self.EPieceType` PieceType))
  (`self.SetDefaultLook` _output_get))

(fn `SetDefaultLook`
  (params (PieceType :type "EPiecesType Enum" :default "E_Bishop"))
  (bind (_returnvalue_x _returnvalue_y) (`KismetMathLibrary.BreakVector` (`self.K2_GetActorLocation`)))
  (bind _staticmeshcomponent (`self.StaticMeshComponent`))
  (bind (_returnvalue_x_2 _returnvalue_y_2 _returnvalue_z) (`KismetMathLibrary.BreakVector` (`SceneComponent.K2_GetComponentLocation` _staticmeshcomponent)))
  (switch `EPiecesType` PieceType
    (:`E_Bishop`
      (set `self.StaticMesh` "/Game/ChessWar/Assets/Bishop.Bishop")
      (set `self.ColorTexture` "/Game/ChessWar/Textures/Bishop/T_Bishop_BaseColor.T_Bishop_BaseColor")
      (set `self.AOTexture` "/Game/ChessWar/Textures/Bishop/T_Bishop_AmbientOcclusion.T_Bishop_AmbientOcclusion")
      (set `self.RoughnessTexture` "/Game/ChessWar/Textures/Bishop/T_Bishop_RoughnessMetallic.T_Bishop_RoughnessMetallic")
      (set `self.NormalTexture` "/Game/ChessWar/Textures/Bishop/T_Bishop_Normal.T_Bishop_Normal")
      (set `self.DecalSize` (72.0 72.0 72.0) :!label _label))
    (:`E_King`
      (set `self.StaticMesh` "/Game/ChessWar/Assets/King.King")
      (set `self.ColorTexture` "/Game/ChessWar/Textures/King/T_King_BaseColor.T_King_BaseColor")
      (set `self.AOTexture` "/Game/ChessWar/Textures/King/T_King_AmbientOcclusion.T_King_AmbientOcclusion")
      (set `self.RoughnessTexture` "/Game/ChessWar/Textures/King/T_King_RoughnessMetallic.T_King_RoughnessMetallic")
      (set `self.NormalTexture` "/Game/ChessWar/Textures/King/T_King_Normal.T_King_Normal")
      (set `self.DecalSize` (93.0 93.0 93.0) :!label _label_2))
    (:`E_Knight`
      (set `self.StaticMesh` "/Game/ChessWar/Assets/Knight.Knight")
      (set `self.ColorTexture` "/Game/ChessWar/Textures/Knight/T_Knight_BaseColor.T_Knight_BaseColor")
      (set `self.AOTexture` "/Game/ChessWar/Textures/Knight/T_Knight_AmbientOcclusion.T_Knight_AmbientOcclusion")
      (set `self.RoughnessTexture` "/Game/ChessWar/Textures/Knight/T_Knight_RoughnessMetallic.T_Knight_RoughnessMetallic")
      (set `self.NormalTexture` "/Game/ChessWar/Textures/Knight/T_Knight_Normal.T_Knight_Normal")
      (goto _label))
    (:`E_Pawn`
      (set `self.StaticMesh` "/Game/ChessWar/Assets/Pawn.Pawn")
      (set `self.ColorTexture` "/Game/ChessWar/Textures/Pawn/T_Pawn_BaseColor.T_Pawn_BaseColor")
      (set `self.AOTexture` "/Game/ChessWar/Textures/Pawn/T_Pawn_AmbientOcclusion.T_Pawn_AmbientOcclusion")
      (set `self.RoughnessTexture` "/Game/ChessWar/Textures/Pawn/T_Pawn_RoughnessMetallic.T_Pawn_RoughnessMetallic")
      (set `self.NormalTexture` "/Game/ChessWar/Textures/Pawn/T_Pawn_Normal.T_Pawn_Normal")
      (set `self.DecalSize` (57.0 57.0 57.0)))
    (:`E_Queen`
      (set `self.StaticMesh` "/Game/ChessWar/Assets/Queen.Queen")
      (set `self.ColorTexture` "/Game/ChessWar/Textures/Queen/T_Queen_BaseColor.T_Queen_BaseColor")
      (set `self.AOTexture` "/Game/ChessWar/Textures/Queen/T_Queen_AmbientOcclusion.T_Queen_AmbientOcclusion")
      (set `self.RoughnessTexture` "/Game/ChessWar/Textures/Queen/T_Queen_RoughnessMetallic.T_Queen_RoughnessMetallic")
      (set `self.NormalTexture` "/Game/ChessWar/Textures/Queen/T_Queen_Normal.T_Queen_Normal")
      (goto _label_2))
    (:`E_Rook`
      (set `self.StaticMesh` "/Game/ChessWar/Assets/Rook.Rook")
      (set `self.ColorTexture` "/Game/ChessWar/Textures/Rook/T_Rook_BaseColor.T_Rook_BaseColor")
      (set `self.AOTexture` "/Game/ChessWar/Textures/Rook/T_Rook_AmbientOcclusion.T_Rook_AmbientOcclusion")
      (set `self.RoughnessTexture` "/Game/ChessWar/Textures/Rook/T_Rook_RoughnessMetallic.T_Rook_RoughnessMetallic")
      (set `self.NormalTexture` "/Game/ChessWar/Textures/Rook/T_Rook_Normal.T_Rook_Normal")
      (set `self.DecalSize` (62.0 62.0 62.0))))
  (`StaticMeshComponent.SetStaticMesh` _staticmeshcomponent (`self.StaticMesh`))
  (bind _returnvalue (`GameplayStatics.SpawnDecalAttached` "/Game/ChessWar/Materials/PostProcess/M_CircleSelection_Decal.M_CircleSelection_Decal" (`self.DecalSize`) (`self.K2_GetRootComponent`) "None" (`KismetMathLibrary.MakeVector` _returnvalue_x _returnvalue_y _returnvalue_z) (struct :`Pitch` -90.0) "KeepWorldPosition"))
  (bind _output_get (set `self.CircleDecal` _returnvalue))
  (`SceneComponent.SetVisibility` _output_get false false)
  (`MaterialInstanceDynamic.SetTextureParameterValue` (`self.Material`) "ColorBaseTexture" (`self.ColorTexture`))
  (`MaterialInstanceDynamic.SetTextureParameterValue` (`self.Material`) "NormalBaseTexture" (`self.NormalTexture`))
  (`MaterialInstanceDynamic.SetTextureParameterValue` (`self.Material`) "AOBaseTexture" (`self.AOTexture`))
  (`MaterialInstanceDynamic.SetTextureParameterValue` (`self.Material`) "RoughnessBaseTexture" (`self.RoughnessTexture`))
  (if (`self.bIsBlack`)
    (`MaterialInstanceDynamic.SetScalarParameterValue` (`self.Material`) "Saturation" 0.8)
    (`MaterialInstanceDynamic.SetVectorParameterValue` (`self.Material`) "Hue" (struct :`R` 0.115 :`G` 0.115 :`B` 0.115 :`A` 1.0)))
  (return))

(fn `SetFantasyLook`
  (params (PieceType :type "EPiecesType Enum" :default "E_Bishop"))
  (bind (_returnvalue_x _returnvalue_y) (`KismetMathLibrary.BreakVector` (`self.K2_GetActorLocation`)))
  (bind _mesh (`self.Mesh`))
  (bind (_returnvalue_x_2 _returnvalue_y_2 _returnvalue_z) (`KismetMathLibrary.BreakVector` (`SceneComponent.K2_GetComponentLocation` (`self.Mesh`))))
  (switch `EPiecesType` PieceType
    (:`E_Bishop`
      _)
    (:`E_King`
      _)
    (:`E_Knight`
      _)
    (:`E_Pawn`
      _)
    (:`E_Queen`
      _)
    (:`E_Rook`
      _))
  (`SkinnedMeshComponent.SetSkinnedAssetAndUpdate` _mesh "/Game/MovementAnimsetPro/UE4_Mannequin/Mesh/SK_Mannequin.SK_Mannequin" true)
  (`SceneComponent.SetWorldScale3D` _mesh (1.3 1.3 1.3))
  (if (`self.bIsBlack`)
    (`MaterialInstanceDynamic.SetVectorParameterValue` (`self.Material`) "BodyColor" (struct :`R` 0.02 :`G` 0.02 :`B` 0.02 :`A` 1.0))
    (`SceneComponent.K2_SetWorldRotation` :`self` _mesh)
    (else
      (`SceneComponent.K2_SetWorldRotation` :`self` _mesh)))
  (set `self.DecalSize` (57.0 57.0 57.0))
  (bind _returnvalue (`GameplayStatics.SpawnDecalAttached` "/Game/ChessWar/Materials/PostProcess/M_CircleSelection_Decal.M_CircleSelection_Decal" (`self.DecalSize`) (`self.K2_GetRootComponent`) "None" (`KismetMathLibrary.MakeVector` _returnvalue_x _returnvalue_y _returnvalue_z) (struct :`Pitch` -90.0) "KeepWorldPosition"))
  (bind _output_get (set `self.CircleDecal` _returnvalue))
  (`SceneComponent.SetVisibility` _output_get false false))

(fn `SetSelected`
  (params (IsSelected :type Boolean))
  (bind _output_get (set `self.bIsSelected` IsSelected))
  (`SceneComponent.SetVisibility` (`self.CircleDecal`) _output_get true))

(fn `UserConstructionScript`)