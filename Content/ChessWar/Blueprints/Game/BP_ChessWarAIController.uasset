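; AI controller for a chess opponent in ChessWar that gathers its color's pieces at BeginPlay and spawns a countdown actor.
; GetBestMove runs a one-ply search, testing each possible move on the live board, scoring it, then undoing it.
; EvaluateBoard sums material and position values, negative for black.
; A recursive alpha-beta MinMax is unfinished and not called here, and an old random-move picker is disconnected.
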(event `self.ReceiveBeginPlay`
  (`|ExecutionSequence`
    (:`then_0`
      (set `self.GameMode` (cast `/Game/ChessWar/Blueprints/Game/BP_ChessWarGameMode` (`GameplayStatics.GetGameMode`) :!pure true)))
    (:`then_1`
      (bind _returnvalue (`|SpawnActorFromClass` "/Game/ChessWar/Blueprints/Game/BP_CountDown.BP_CountDown_C" (`KismetMathLibrary.MakeTransform` (0.0 0.0 0.0)) "Undefined" "OverrideRootScale" null null))
      (set `self.CountDown` _returnvalue))
    (:`then_2`
      (bind _outactors (`GameplayStatics.GetAllActorsOfClass` "/Game/ChessWar/Blueprints/Game/BP_ChessWarCharacter.BP_ChessWarCharacter_C"))
      (for _array_element _outactors
        (bind _asbp_chess_war_character (cast `/Game/ChessWar/Blueprints/Game/BP_ChessWarCharacter` _array_element :!pure true))
        (if (== (`self.Color`) (`KismetMathLibrary.Conv_BoolToByte` (not (`ChessWarCharacter.bIsBlack` _asbp_chess_war_character))))
          (`KismetArrayLibrary.Array_AddUnique` (`self.PossesedPieces`) _asbp_chess_war_character))))))

(fn `EvaluateBoard`
  (params (Board :type "/Game/ChessWar/Blueprints/Game/BP_Board Object Reference"))
  (returns (Evaluation :type "Float (double-precision)"))
  (locals (PieceValue :type "Float (double-precision)") (TotalEValuation :type "Float (double-precision)"))
  (set `local.TotalEvaluation` 0.0)
  (for _array_element (`Board.TPieces` Board)
    (bind _asbp_chess_war_character (cast `/Game/ChessWar/Blueprints/Game/BP_ChessWarCharacter` _array_element :!pure true))
    (bind _epiecetype (`ChessWarCharacter.EPieceType` _asbp_chess_war_character))
    (switch `EPiecesType` _epiecetype
      (:`E_Bishop`
        (bind _bisblack (`ChessWarCharacter.bIsBlack` _asbp_chess_war_character))
        (bind (_findexposition_x _findexposition_y) (`KismetMathLibrary.BreakVector2D` (`/Game/ChessWar/Blueprints/Game/BP_ChessWarCharacter.FIndexPosition` _asbp_chess_war_character)))
        (bind _returnvalue (`self.GetEvaluationByPieceType` _epiecetype _bisblack (`KismetMathLibrary.FTrunc` _findexposition_x) (`KismetMathLibrary.FTrunc` _findexposition_y)))
        (set `local.PieceValue` (+ 30.0 _returnvalue)))
      (:`E_King`
        (set `local.PieceValue` (+ 900.0 _returnvalue)))
      (:`E_Knight`
        (set `local.PieceValue` (+ 30.0 _returnvalue)))
      (:`E_Pawn`
        (set `local.PieceValue` (+ 10.0 _returnvalue)))
      (:`E_Queen`
        (set `local.PieceValue` (+ 90.0 _returnvalue)))
      (:`E_Rook`
        (set `local.PieceValue` (+ 50.0 _returnvalue))))
    (if _bisblack
      (set `local.PieceValue` (* -1 (`local.PieceValue`))))
    (set `local.TotalEvaluation` (+ (`local.PieceValue`) (`local.TotalEvaluation`))))
  (return (`local.TotalEValuation`)))

(fn `GetBestMove`
  (returns (Piece :type "/Game/ChessWar/Blueprints/Game/BP_ChessWarCharacter Object Reference") (NewPosX :type "Float (double-precision)") (NewPosY :type "Float (double-precision)"))
  (locals (PiecesWithPossibleMovement :type "Array of /Game/ChessWar/Blueprints/Game/BP_ChessWarCharacter Object Reference") (BestPiece :type "/Game/ChessWar/Blueprints/Game/BP_ChessWarCharacter Object Reference") (BestMove :type "Vector2D Structure") (BoardValue :type "Float (double-precision)") (BestValue :type "Float (double-precision)" :default -9999.0) (Board :type "/Game/ChessWar/Blueprints/Game/BP_Board Object Reference") (SelectedMove :type "Vector2D Structure"))
  (bind (_selectedmove_x _selectedmove_y) (`KismetMathLibrary.BreakVector2D` (`local.SelectedMove`)))
  (bind (_bestmove_x _bestmove_y) (`KismetMathLibrary.BreakVector2D` (`local.BestMove`)))
  (for _array_element (`self.PossesedPieces`)
    ;[1 1 1] Si la piece est toujours en jeu sinon c'est qu'elle a été mangée, on la supprime
    (`/Engine/EditorBlueprintResources/StandardMacros.IsValid` _array_element
      (:`Is Valid`
        (if (!= (`KismetArrayLibrary.Array_Length` (`ChessWarCharacter.TPossiblePositions` _array_element)) 0)
          (bind _output_get (set `self.SelectedPiece` _array_element))
          (for _array_element_2 (`ChessWarCharacter.TPossiblePositions` _output_get)
            (set `local.selectedMove` (`KismetMathLibrary.MakeVector2D` (`KismetMathLibrary.BreakVector2D` _array_element_2) (`.Y` (`KismetMathLibrary.BreakVector2D` _array_element_2))))
            (bind _output_get_2 (set `local.Board` (`/Game/ChessWar/Blueprints/Game/BP_ChessWarGameMode.Board` (`self.GameMode`))))
            (bind _capturedpiece (`self.TestMove` _output_get_2 (`self.SelectedPiece`) _selectedmove_x _selectedmove_y))
            (bind _evaluation (`self.EvaluateBoard` (`local.Board`)))
            (set `local.BoardValue` _evaluation)
            (if (`ChessWarCharacter.bIsBlack` (`self.SelectedPiece`))
              (set `local.BoardValue` (* -1 (`local.BoardValue`))))
            (`self.UndoMove` (`local.Board`) _capturedpiece)
            (if (> (`local.BoardValue`) (`local.BestValue`))
              (set `local.BestValue` (`local.BoardValue`))
              (set `local.BestPiece` (`self.SelectedPiece`))
              (set `local.BestMove` (`local.selectedMove`))))))
      (:`Is Not Valid`
        (`KismetArrayLibrary.Array_RemoveItem` (`self.PossesedPieces`)))))
  (return (`local.BestPiece`) _bestmove_x _bestmove_y))

(fn `MinMax`
  (params (Board :type "/Game/ChessWar/Blueprints/Game/BP_Board Object Reference") (Depth :type "Float (double-precision)") (Alpha :type "Float (double-precision)") (Beta :type "Float (double-precision)") (Color :type "/Game/ChessWar/Blueprints/Game/EColor Enum" :default "NewEnumerator0"))
  (returns (Value :type "Float (double-precision)"))
  (locals (BestValue :type "Float (double-precision)") (LDepth :type "Float (double-precision)") (LBeta :type "Float (double-precision)") (LBoard :type "/Game/ChessWar/Blueprints/Game/BP_Board Object Reference") (LAlpha :type "Float (double-precision)"))
  (set `local.LBoard` Board)
  (set `local.LDepth` Depth)
  (set `local.LAlpha` Alpha)
  (set `local.LBeta` Beta)
  (if (== Depth 0.0)
    (bind _evaluation (`self.EvaluateBoard` (`local.LBoard`)))
    (return _evaluation)
    (elif (== Color (`self.Color`))
      (set `local.BestValue` 9999.0)
      (for _array_element (`Board.TPieces` (`local.LBoard`))
        (bind _asbp_chess_war_character (cast `/Game/ChessWar/Blueprints/Game/BP_ChessWarCharacter` _array_element :!pure true))
        (if (or (and (not (`ChessWarCharacter.bIsBlack` _asbp_chess_war_character)) (`|EnumInequality` (`self.Color`) "NewEnumerator0")) (and (`ChessWarCharacter.bIsBlack` _asbp_chess_war_character) (`|EnumInequality` (`self.Color`) "NewEnumerator1")))
          (if (!= (`KismetArrayLibrary.Array_Length` (`ChessWarCharacter.TPossiblePositions` _asbp_chess_war_character)) 0)
            (bind _output_get (set `self.SelectedPiece` _asbp_chess_war_character))
            (for _array_element_2 (`ChessWarCharacter.TPossiblePositions` _output_get)
              (bind _capturedpiece (`self.TestMove` (`local.LBoard`) (`self.SelectedPiece`) (`KismetMathLibrary.BreakVector2D` _array_element_2) (`.Y` (`KismetMathLibrary.BreakVector2D` _array_element_2))))
              (bind _result (`/Engine/EditorBlueprintResources/StandardMacros.DecrementFloat` (`local.LDepth`))
                (:`  `
                  (bind _value (`self.MinMax` (`local.LBoard`) _result (`local.LAlpha`) (`local.LBeta`) (`self.Color`)))
                  (set `local.BestValue` (`KismetMathLibrary.FMin` _value (`local.BestValue`)))
                  (`self.UndoMove` (`local.LBoard`) _capturedpiece)
                  (bind _output_get_2 (set `local.LBeta` (`KismetMathLibrary.FMin` (`local.LBeta`) (`local.LAlpha`))))
                  (if (<= _output_get_2 (`local.LAlpha`))
                    (return (`local.BestValue`)))))))))
      (else
        (set `local.BestValue` -9999.0)))))

(fn `TestMove`
  (params (Board :type "/Game/ChessWar/Blueprints/Game/BP_Board Object Reference") (SelectedPiece :type "/Game/ChessWar/Blueprints/Game/BP_ChessWarCharacter Object Reference") (TargetX :type "Float (double-precision)") (TargetY :type "Float (double-precision)"))
  (returns (CapturedPiece :type "ChessWarCharacter Object Reference"))
  (locals (BPBoard :type "/Game/ChessWar/Blueprints/Game/BP_Board Object Reference"))
  (bind (_returnvalue_x _returnvalue_y _returnvalue_z) (`KismetMathLibrary.BreakVector` (`self.K2_GetActorLocation` SelectedPiece)))
  (bind _bpboard (`local.BPBoard`))
  (bind _output_get (set `local.BPBoard` Board))
  (`/Game/ChessWar/Blueprints/Game/BP_Board.MoveSelectedPiece` _output_get SelectedPiece TargetX TargetY _returnvalue_z)
  (bind _output_get_2 (set `/Game/ChessWar/Blueprints/Game/BP_Board.CapturedPiece` (`Board.GetPieceToCaptureOnTarget` _bpboard) _bpboard))
  (`/Game/ChessWar/Blueprints/Game/BP_Board.CapturePieceOnTarget` _bpboard false)
  (return _output_get_2))

(fn `UndoMove`
  (params (Board :type "/Game/ChessWar/Blueprints/Game/BP_Board Object Reference") (CapturedPiece :type "ChessWarCharacter Object Reference (by ref)"))
  (locals (BPBoard :type "/Game/ChessWar/Blueprints/Game/BP_Board Object Reference") (BPCapturedPiece :type "ChessWarCharacter Object Reference"))
  (bind _selectedpiece (`self.SelectedPiece`))
  (bind _bpcapturedpiece (`local.BPCapturedPiece`))
  (bind (_returnvalue_x _returnvalue_y _returnvalue_z) (`KismetMathLibrary.BreakVector` (`self.K2_GetActorLocation` _selectedpiece)))
  (bind (_fpreviousposition_x _fpreviousposition_y) (`KismetMathLibrary.BreakVector2D` (`/Game/ChessWar/Blueprints/Game/BP_ChessWarCharacter.FPreviousPosition` _selectedpiece)))
  (set `local.BPBoard` Board)
  (set `local.BPCapturedPiece` CapturedPiece)
  (`/Game/ChessWar/Blueprints/Game/BP_Board.SetPieceLocationAndUpdatePieceDatas` (`local.BPBoard`) _selectedpiece _fpreviousposition_x _fpreviousposition_y _returnvalue_z)
  (`/Engine/EditorBlueprintResources/StandardMacros.IsValid` _bpcapturedpiece
    (:`Is Valid`
      (`KismetArrayLibrary.Array_Add` (`Board.TPieces` (`local.BPBoard`)) _bpcapturedpiece))))

(fn `UserConstructionScript`)