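; Player pawn for a tic-tac-toe game (TTT) that places round or cross marks as Paper2D flipbook components and presents each round's result.
; Mouse clicks and AIPlay both feed PlayTurn, which fills an empty cell with a randomly chosen flipbook variant, checks for victory and asks the GameMode to change turn.
; OnDeclareWinner shows draw or winner text, adds an oriented winning-line flipbook, then clears the board.
; BeginPlay reads AI difficulty from custom config.
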(event `self.ReceiveBeginPlay`
  ;[1 1 1] Multicast On Begin Event
  (`|ExecutionSequence`
    (:`then_0`
      (switch `string` (`self.GetCustomConfigVar_String` "Game Rules" "DifficultyText")
        (:`Easy`
          (set `self.LevelOfDifficulty` 1))
        (:`Medium`
          (set `self.LevelOfDifficulty` 3))
        (:`Hard`
          (set `self.LevelOfDifficulty` 5))))
    (:`then_1`
      (bind _asbp_game_state (cast `` (`GameplayStatics.GetGameState`)))
      (set `self.GameState` _asbp_game_state))
    (:`then_2`
      (bind _asbp_game_mode (cast `` (`GameplayStatics.GetGameMode`)))
      (set `self.GameMode` _asbp_game_mode))))

(event `self.OnDeclareWinner`
  (params (IsDraw :type Boolean) (FirstRow :type Integer) (FirstColumn :type Integer) (Direction :type String))
  (bind _gamemode (`self.GameMode`))
  (bind _gamehud (`self.GameHUD`))
  ;[1 1 1] Is Winner / Draw Event
  (if IsDraw
    (`self.DisplayGameInfos` (`self.GameHUD`) "DRAW")
    (`KismetSystemLibrary.Delay` 1.8)
    (`self.Clear Game Board`)
    (else
      (bind _returnvalue (`self.GetXYInPixelFromArrayPosition` FirstRow FirstColumn))
      (`KismetSystemLibrary.Delay` 0.2)
      (set `self.PosXYInPixel` _returnvalue)
      (bind _returnvalue_2 (`AddComponent|PaperFlipbookComponent_4`))
      (`KismetArrayLibrary.Array_Add` (`self.FlipbookComponents`) _returnvalue_2)
      (set `self.FlipbookComponent` _returnvalue_2)
      (switch `string` Direction
        (:`DR`
          (`self.Set Flipbook Position` (`self.FlipbookComponent`) (`self.PosXYInPixel`) 80.0 50.0 -100.0 1.0))
        (:`DL`
          (`self.Set Flipbook Position` (`self.FlipbookComponent`) (`self.PosXYInPixel`) -80.0 80.0 0.0 1.0))
        (:`V`
          (`self.Set Flipbook Position` (`self.FlipbookComponent`) (`self.PosXYInPixel`) 5.0 90.0 -50.0 0.7))
        (:`H`
          (`self.Set Flipbook Position` (`self.FlipbookComponent`) (`self.PosXYInPixel`) -100.0 0.0 40.0 0.8)))
      (`GameplayStatics.PlaySoundAtLocation` null (0.0 0.0 0.0) 1.5)
      (`self.SetPoints` _gamemode)
      (if (!= (`/Game/ChessWar/Blueprints/Game/_TTT/BP_PlayerPawn.CurrentPlayerWinner` _gamemode) (`/Game/ChessWar/Blueprints/Game/_TTT/BP_PlayerPawn.CurrentPlayer` _gamemode))
        (switch `|SwitchEnum` (`/Game/ChessWar/Blueprints/Game/_TTT/BP_PlayerPawn.GameType` (`self.GameMode`))
          (:`NewEnumerator1`
            (`self.DisplayGameInfos` _gamehud "COMPUTER WIN"))
          (:`NewEnumerator0`
            (`self.DisplayGameInfos` _gamehud (`KismetTextLibrary.Conv_StringToText` (`KismetStringLibrary.BuildString_Int` "" "PLAYER  " (`/Game/ChessWar/Blueprints/Game/_TTT/BP_PlayerPawn.Turn` (`self.GameState`)) " WIN")) :!label _label)))
        (else
          (goto _label)))
      (`KismetSystemLibrary.Delay` 1.8)
      (`self.Clear Game Board`))))

(event `self.ReceiveActorOnClicked`
  ;[1 1 1] Game Turn On Click Event
  (bind (_posx _posy _centerpositionsinpixel) (`self.GetPositionUnderMouse` 6 -8))
  (`self.PlayTurn` _centerpositionsinpixel _posx _posy))

(event `AIPlay`
  (params (PosX :type Integer) (PosY :type Integer))
  ;[1 1 1] Game Turn For AI
  (`KismetSystemLibrary.Delay` 0.2) ; Créer une variable pour ça
  (bind _returnvalue (`self.GetPositionInPixelWithPosXAndPoxY` PosX PosY 6 -8))
  (`self.PlayTurn` _returnvalue PosX PosY))

(event `self.ReceivePossessed`
  (params (NewController :type "Controller Object Reference"))
  (bind _gamestate (`self.GameState`))
  ;[1 1 1] OnEventPossessed - change figure for current player
  (bind _asbp_player_controller (cast `` NewController))
  (set `self.CurentPlayer` _asbp_player_controller)
  (if (== (`/Game/ChessWar/Blueprints/Game/_TTT/BP_PlayerPawn.PaperFilpbookType` _asbp_player_controller) 0)
    (set `/Game/ChessWar/Blueprints/Game/_TTT/BP_PlayerPawn.PlayerFigure` null _gamestate)
    (else
      (set `/Game/ChessWar/Blueprints/Game/_TTT/BP_PlayerPawn.PlayerFigure` null _gamestate))))

(fn `Clear Game Board`
  (`self.ClearBoard`)
  (for _array_element (`self.FlipbookComponents`)
    (`ActorComponent.K2_DestroyComponent` _array_element)))

(fn `PlayTurn`
  (params (PosXYInPixel :type "Vector Structure") (PosX :type Integer) (PosY :type Integer))
  (locals (FlipBook :type "PaperFlipbook Object Reference"))
  (bind _turn (`/Game/ChessWar/Blueprints/Game/_TTT/BP_PlayerPawn.Turn` (`self.GameState`)))
  (set `self.PosXYInPixel` PosXYInPixel)
  (if (`self.IsCellEmpty` PosX PosY)
    (`GameplayStatics.PlaySoundAtLocation` null)
    (bind _returnvalue (`AddComponent|PaperFlipbookComponent_6`))
    (`self.GetPaperFlipbookType`
      (:`Round`
        (switch `int` (`KismetMathLibrary.RandomIntegerInRange` 0 4)
          (:`0`
            (set `local.FlipBook` null))
          (:`1`
            (set `local.FlipBook` null))
          (:`2`
            (set `local.FlipBook` null))
          (:`3`
            (set `local.FlipBook` null))
          (:`4`
            (set `local.FlipBook` null))))
      (:`Cross`
        (switch `int` (`KismetMathLibrary.RandomIntegerInRange` 0 3)
          (:`0`
            (set `local.FlipBook` null))
          (:`1`
            (set `local.FlipBook` null))
          (:`2`
            (set `local.FlipBook` null))
          (:`3`
            (set `local.FlipBook` null)))))
    (`PaperFlipbookComponent.SetFlipbook` _returnvalue (`local.FlipBook`))
    (`KismetArrayLibrary.Array_Add` (`self.FlipbookComponents`) _returnvalue)
    (`self.Set Flipbook Position` _returnvalue (`self.PosXYInPixel`) 0.0 0.0 0.0 1.0 false (struct :`R` 1.0 :`G` 1.0 :`B` 1.0 :`A` 1.0))
    (`self.SetTurnInCell` PosX PosY _turn)
    (bind _returnvalue_2 (`self.CheckVictory` _turn))
    (`self.ChangeTurn` (`self.GameMode`) (or _returnvalue_2 (`self.IsBoardFull`)))))

(fn `Set Flipbook Position`
  (params (FlipbookComponent :type "PaperFlipbookComponent Object Reference") (VectorPosition :type "Vector Structure") (BalancingX :type "Float (double-precision)") (BalancingZ :type "Float (double-precision)") (PitchRotation :type "Float (double-precision)") (Scale :type "Float (double-precision)") (Looping :type Boolean) (`Sprite Color` :type "LinearColor Structure"))
  (locals (Flipbook :type "PaperFlipbookComponent Object Reference"))
  (set `local.Flipbook` FlipbookComponent)
  (`PaperFlipbookComponent.SetLooping` (`local.Flipbook`) Looping)
  (`SceneComponent.K2_SetWorldLocation` (`local.Flipbook`) (+ VectorPosition (`KismetMathLibrary.MakeVector` BalancingX 0.0 BalancingZ)) false)
  (`SceneComponent.K2_SetWorldRotation` (`local.Flipbook`) (`KismetMathLibrary.MakeRotator` PitchRotation) false)
  (`SceneComponent.SetWorldScale3D` (`local.Flipbook`) (`KismetMathLibrary.MakeVector` Scale Scale Scale)))

(fn `UserConstructionScript`)