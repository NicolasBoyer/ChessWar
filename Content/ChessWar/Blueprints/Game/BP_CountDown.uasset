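; BP_CountDown is the countdown timer for ChessWar, tracking remaining time and a short formatted time string.
; Initialize reads the enable flag and minute-based duration from BP_ChessWarGameInstance, converting the duration to seconds.
; While enabled and playing, Tick accumulates elapsed time and refreshes both values, with no clamp or expiry event at zero.
; Play and Pause toggle ticking progress; Stop also clears elapsed time, without refreshing the displayed values.
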(event `Initialize`
  (bind _returnvalue (* (`self.TimeDuration`) 60.0))
  (bind _asbp_chess_war_game_instance (cast `/Game/ChessWar/Blueprints/Game/BP_ChessWarGameInstance` (`GameplayStatics.GetGameInstance`) :!pure true))
  ;[1 1 1] IsCountDown And get Time Duration
  (set `self.TimeDuration` (`/Game/ChessWar/Blueprints/Game/BP_ChessWarGameInstance.CountDownDuration` _asbp_chess_war_game_instance))
  (bind _output_get (set `self.IsCountDown` (`/Game/ChessWar/Blueprints/Game/BP_ChessWarGameInstance.IsCountDown` _asbp_chess_war_game_instance)))
  (if _output_get
    (set `self.CurrentFormatTime` (`KismetStringLibrary.GetSubstring` (`KismetStringLibrary.TimeSecondsToString` _returnvalue) 0 5)))
  (set `self.CurrentTimeSec` _returnvalue))

(event `self.ReceiveTick`
  (params (DeltaSeconds :type "Float (single-precision)"))
  ;[1 1 1] GetAndSetCurrentTime
  (if (and (`self.IsCountDown`) (`self.IsPlaying`))
    (bind _output_get (set `self.ElapsedTime` (+ DeltaSeconds (`self.ElapsedTime`))))
    (bind _returnvalue (- (* (`self.TimeDuration`) 60.0) _output_get))
    (set `self.CurrentTimeSec` _returnvalue)
    (set `self.CurrentFormatTime` (`KismetStringLibrary.GetSubstring` (`KismetStringLibrary.TimeSecondsToString` _returnvalue) 0 5))))

(event `Event Pause`
  ;[1 1 1] API
  (set `self.IsPlaying` false))

(event `Event Play`
  ;[1 1 1] API
  (set `self.IsPlaying` true))

(event `Event Stop`
  ;[1 1 1] API
  (set `self.IsPlaying` false)
  (set `self.ElapsedTime` 0.0))

(fn `UserConstructionScript`)